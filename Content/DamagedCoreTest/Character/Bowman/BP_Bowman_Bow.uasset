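; Bowman's bow actor, which draws a two-segment string and fires projectiles, with optional fire and multi-shot modes.
; UpdateString stretches both segments to the pull point, spawns arrows once per draw past a small threshold, and keeps them aimed through the bow.
; ReleaseString launches arrows at speed proportional to pull distance, ignoring owner and other projectiles.
; A timeline snaps the string back to rest, then re-arms spawning.
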(event Custom|UpdateString
  (params (CenterPosition :type Vector))
  (bind _returnvalue (* 1.0 0.003))
  (bind _end2 (Variables|Default|Getend2))
  (bind _end1 (Variables|Default|Getend1))
  (bind _returnvalue_2 (Transformation|GetWorldLocation _end2))
  (bind _returnvalue_3 (Transformation|GetWorldLocation _end1))
  (Utilities|FlowControl|Sequence
    (:then_0
      ;[1 1 1] update the string
      (Transformation|SetWorldTransform (Variables|Default|Getstring2) (Math|Transform|MakeTransform (* (+ CenterPosition _returnvalue_2) 0.5) (Math|Rotator|FindLookatRotation CenterPosition _returnvalue_2) (Math|Vector|MakeVector (* (Math|Vector|VectorLength (- CenterPosition _returnvalue_2)) 0.01) _returnvalue _returnvalue)) false false)
      (Transformation|SetWorldTransform (Variables|Default|Getstring1) (Math|Transform|MakeTransform (* (+ CenterPosition _returnvalue_3) 0.5) (Math|Rotator|FindLookatRotation CenterPosition _returnvalue_3) (Math|Vector|MakeVector (* (Math|Vector|VectorLength (- CenterPosition _returnvalue_3)) 0.01) _returnvalue _returnvalue)) false false))
    (:then_1
      ;[1 1 1] update the arrow
      (if (> (Math|Vector|VectorLength (- CenterPosition (* (+ (Transformation|GetWorldLocation (Variables|Default|Getend1)) (Transformation|GetWorldLocation (Variables|Default|Getend2))) 0.5))) 15.0)
        (Utilities|FlowControl|DoOnce false
          (:Completed
            (CallFunction|SpawnArrow CenterPosition)))))
    (:then_2
      (CallFunction|UpdateArrow CenterPosition))))

(event Custom|ResetArrowSpawn
  ;[1 1 1] update the arrow
  (Utilities|FlowControl|DoOnce false) ; enters at Reset
)

(event Custom|SpawnArrow
  (params (HandPosition :type Vector))
  (bind _self self)
  (bind _self_2 self)
  (bind _returnvalue (Components|GetOwner _self_2))
  (bind _returnvalue_2 (Components|GetOwner _self))
  (bind _aspawn (Utilities|Casting|CastToPawn _returnvalue_2))
  (bind _aspawn_2 (Utilities|Casting|CastToPawn _returnvalue))
  (if (Variables|Default|GetNextShotIsMultiShot)
    (for _array_element (Variables|Default|GetMutliShotXOffset)
      (bind _returnvalue_3 (Game|SpawnActorfromClass "/Game/DamagedCoreTest/Weapon/Bullet/BowmanProjectile.BowmanProjectile_C" (Math|Transform|MakeTransform HandPosition (Math|Rotator|FindLookatRotation HandPosition (Math|Transform|TransformLocation (Transformation|GetActorTransform) (Math|Vector|MakeVector _array_element 0.0 0.0))) "2.000000,2.000000,2.000000") "Undefined" _aspawn (Variables|Default|GetNextShotIsOnFire) _aspawn))
      (Actor|SetLifeSpan _returnvalue_3 0.0)
      (Utilities|Array|Add (Variables|Default|GetSpawnedArrows) _returnvalue_3))
    (else
      (bind _returnvalue_4 (Game|SpawnActorfromClass "/Game/DamagedCoreTest/Weapon/Bullet/BowmanProjectile.BowmanProjectile_C" (Math|Transform|MakeTransform HandPosition (Math|Rotator|FindLookatRotation HandPosition (Transformation|GetActorLocation)) "2.000000,2.000000,2.000000") "Undefined" _aspawn_2 (Variables|Default|GetNextShotIsOnFire) _aspawn_2))
      (Actor|SetLifeSpan _returnvalue_4 0.0)
      (Utilities|Array|Add (Variables|Default|GetSpawnedArrows) _returnvalue_4)))
  (Variables|Default|SetNextShotIsOnFire false)
  (Rendering|Material|SetScalarParameterValueonMaterials (Variables|Default|GetBowMesh) "ChangeColor" 0.0))

(event Custom|UpdateArrow
  (params (HandPosition :type Vector))
  (bind _spawnedarrows (Variables|Default|GetSpawnedArrows))
  (if (Variables|Default|GetNextShotIsMultiShot)
    (if (> (Utilities|Array|Length (Variables|Default|GetSpawnedArrows)) 0)
      (for (_array_element _array_index) (Variables|Default|GetMutliShotXOffset)
        (Transformation|SetActorTransform (Utilities|Array|Get(acopy) (Variables|Default|GetSpawnedArrows) _array_index) (Math|Transform|MakeTransform HandPosition (Math|Rotator|FindLookatRotation HandPosition (Math|Transform|TransformLocation (Transformation|GetActorTransform) (Math|Vector|MakeVector _array_element 0.0 0.0))) "2.000000,2.000000,2.000000"))))
    (elif (> (Utilities|Array|Length _spawnedarrows) 0)
      (Transformation|SetActorTransform (Utilities|Array|Get(acopy) _spawnedarrows) (Math|Transform|MakeTransform HandPosition (Math|Rotator|FindLookatRotation HandPosition (Transformation|GetActorLocation)) "2.000000,2.000000,2.000000")))))

(event Custom|ReleaseString
  (params (ReleasePosition :type Vector))
  (bind _spawnedarrows (Variables|Default|GetSpawnedArrows))
  (Utilities|FlowControl|Sequence
    (:then_0
      ;[1 1 1] shoot arrow if have
      (Variables|Default|SetNextShotIsMultiShot false)
      (for _array_element _spawnedarrows
        (Transformation|DetachFromActor _array_element "KeepWorld" "KeepWorld" "KeepWorld")
        (Variables|/Script/Engine.MovementComponent|SetVelocity (Variables|/Game/DamagedCoreTest/Weapon/Bullet/BowmanProjectile.BowmanProjectile_C|GetProjectileMovement _array_element) (* (Math|Vector|GetForwardVector (Variables|/Game/DamagedCoreTest/Weapon/Bullet/BowmanProjectile.BowmanProjectile_C|GetStaticMesh _array_element)) (Math|Vector|VectorLength (* (- (* (+ (Transformation|GetWorldLocation (Variables|Default|Getend1)) (Transformation|GetWorldLocation (Variables|Default|Getend2))) 0.5) ReleasePosition) 5e+01))))
        (Components|Activation|SetActive (Variables|/Game/DamagedCoreTest/Weapon/Bullet/BowmanProjectile.BowmanProjectile_C|GetProjectileMovement _array_element) true false)
        (Actor|SetLifeSpan _array_element 5.0)
        (Collision|IgnoreActorwhenMoving (Variables|/Game/DamagedCoreTest/Weapon/Bullet/BowmanProjectile.BowmanProjectile_C|GetStaticMesh _array_element) (Components|GetOwner self) true)
        (bind _outactors (Actor|GetAllActorsOfClass "/Game/DamagedCoreTest/Weapon/Bullet/BowmanProjectile.BowmanProjectile_C"))
        (for _array_element_2 _outactors
          (Collision|IgnoreActorwhenMoving (Variables|/Game/DamagedCoreTest/Weapon/Bullet/BowmanProjectile.BowmanProjectile_C|GetStaticMesh _array_element) _array_element_2 true)))
      (Utilities|Array|Clear _spawnedarrows))
    (:then_1
      ;[1 1 1] update string
      (bind _lerp (Timeline|ReleaseStringTimeLine PlayFromStart)
        (:Update
          (CallFunction|UpdateString (Math|Vector|Lerp(Vector) ReleasePosition (* (+ (Transformation|GetWorldLocation (Variables|Default|Getend1)) (Transformation|GetWorldLocation (Variables|Default|Getend2))) 0.5) _lerp)))
        (:Finished
          (CallFunction|ResetArrowSpawn))))))

(event Custom|SetNextShotIsMultiShot
  (Variables|Default|SetNextShotIsMultiShot true))

(event Custom|SetNextShotIsOnFire
  (Variables|Default|SetNextShotIsOnFire true)
  (Rendering|Material|SetScalarParameterValueonMaterials (Variables|Default|GetBowMesh) "ChangeColor" 1.0))

(fn ConstructionScript
  (CallFunction|UpdateString (* (+ (Transformation|GetWorldLocation (Variables|Default|Getend1)) (Transformation|GetWorldLocation (Variables|Default|Getend2))) 0.5)))