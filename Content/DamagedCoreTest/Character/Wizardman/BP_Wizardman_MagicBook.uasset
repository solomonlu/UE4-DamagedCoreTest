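; Wizardman's magic book, a skeletal mesh Blueprint whose animation runs forward or in reverse depending on whether it is the red book.
; ToggleBook flips the IsRedBook flag.
; Every Tick casts the mesh's anim instance to SKM_MagicBook_AnimBlueprint and sets its PlayRate sign from that flag, reversing playback while the book is red.
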(event Custom|ToggleBook
  (Variables|Default|SetIsRedBook (not (Variables|Default|GetIsRedBook))))

(event EventTick
  (params (DeltaSeconds :type Float%20%28single-precision%29))
  (if (not (Variables|Default|GetIsRedBook))
    (Variables|/Game/DamagedCoreTest/SkeletalMesh/MagicBook/SKM_MagicBook_AnimBlueprint.SKM_MagicBook_AnimBlueprint_C|SetPlayRate (.AsSKM%20Magic%20Book%20Anim%20Blueprint (Utilities|Casting|CastToSKM_MagicBook_AnimBlueprint (Components|SkeletalMesh|GetAnimInstance (Variables|Default|GetSkeletalMesh)))) 1.0)
    (else
      (Variables|/Game/DamagedCoreTest/SkeletalMesh/MagicBook/SKM_MagicBook_AnimBlueprint.SKM_MagicBook_AnimBlueprint_C|SetPlayRate (.AsSKM%20Magic%20Book%20Anim%20Blueprint (Utilities|Casting|CastToSKM_MagicBook_AnimBlueprint (Components|SkeletalMesh|GetAnimInstance (Variables|Default|GetSkeletalMesh)))) -1.0))))

(fn ConstructionScript)