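; Wizardman's magic stick, which absorbs nearby magic balls and launches them as a single projectile.
; While absorbing, Tick pulls balls overlapping AbsorbSphere inward, faster as they get closer, and absorbs those that reach its center, up to a small cap.
; The first ball spawns a projectile attached to the stick; later ones enlarge it and add their color.
; Stopping absorption detaches and launches the projectile along the scaled right-hand velocity, ignoring the owner.
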(event Custom|StartAbsorbMagicBall
  (Variables|Default|SetIsAbsorbingMagicBall true))

(event Custom|DoAbsorbOneMagicBall
  (params (MagicBall :type Wizardman%20Magic%20Ball%20Object%20Reference))
  (bind _isred (Variables|/Game/DamagedCoreTest/Weapon/Bullet/WizardmanMagicBall.WizardmanMagicBall_C|GetIsRed MagicBall))
  (Math|Integer|IncrementInt (Variables|Default|GetAbsorbedCount)
    (:%20%20
      (Utilities|IsValid (Variables|Default|GetSpawnedProjectile)
        (:Is%20Valid
          ;[1 1 1] if already have a ball on the stick,scale it
          (Transformation|SetActorScale3D (Variables|Default|GetSpawnedProjectile) (* (Transformation|GetActorScale3D (Variables|Default|GetSpawnedProjectile)) 2.0))
          (Default|AddNewMagicBall (Variables|Default|GetSpawnedProjectile) _isred))
        (:Is%20Not%20Valid
          ;[1 1 1] if no ball on the stick,spawn it
          (bind _returnvalue (Game|SpawnActorfromClass "/Game/DamagedCoreTest/Weapon/Bullet/WizardmanProjectile.WizardmanProjectile_C" (Math|Transform|MakeTransform "0.0,0.0,100.000000" "0, 0, 0" "0.750000,0.750000,0.750000") "AdjustIfPossibleButAlwaysSpawn" (Components|GetOwner self) _isred 0))
          (bind _output_get (Variables|Default|SetSpawnedProjectile _returnvalue))
          (Transformation|AttachComponentToComponent _output_get (Variables|Default|GetStaticMesh) "None" "KeepRelative" "KeepRelative" "KeepWorld" true)
          (Actor|SetLifeSpan _returnvalue 0.0))))))

(event Custom|StopAbsorbMagicBall
  (params (RightHandVelocity :type Vector))
  (Variables|Default|SetIsAbsorbingMagicBall false)
  (Utilities|IsValid (Variables|Default|GetSpawnedProjectile)
    (:Is%20Valid
      (Transformation|DetachFromActor (Variables|Default|GetSpawnedProjectile) "KeepWorld" "KeepWorld" "KeepWorld")
      (Variables|/Script/Engine.MovementComponent|SetVelocity (Variables|/Game/DamagedCoreTest/Weapon/Bullet/WizardmanProjectile.WizardmanProjectile_C|GetProjectileMovement (Variables|Default|GetSpawnedProjectile)) (* RightHandVelocity 5.0))
      (Collision|IgnoreActorwhenMoving (Variables|/Game/DamagedCoreTest/Weapon/Bullet/WizardmanProjectile.WizardmanProjectile_C|GetCollisionComponent (Variables|Default|GetSpawnedProjectile)) (Components|GetOwner self) true)
      (Components|Activation|SetActive (Variables|/Game/DamagedCoreTest/Weapon/Bullet/WizardmanProjectile.WizardmanProjectile_C|GetProjectileMovement (Variables|Default|GetSpawnedProjectile)) true false)
      (Default|ReleasefromHand (Variables|Default|GetSpawnedProjectile))
      (Variables|Default|SetSpawnedProjectile 0)
      (Variables|Default|SetAbsorbedCount 0))))

(event EventTick
  (params (DeltaSeconds :type Float%20%28single-precision%29))
  (if (< (Variables|Default|GetAbsorbedCount) 3)
    ;[1 1 1] if close enough then absorb,if not then try attract
    (if (Variables|Default|GetIsAbsorbingMagicBall)
      (for _array_element (Collision|GetOverlappingActors (Variables|Default|GetAbsorbSphere) "/Game/DamagedCoreTest/Weapon/Bullet/WizardmanMagicBall.WizardmanMagicBall_C" :!class /Script/Engine.PrimitiveComponent)
        (if (< (Math|Vector|VectorLength (- (Transformation|GetWorldLocation (Variables|Default|GetAbsorbSphere)) (Transformation|GetActorLocation (.AsWizardman%20Magic%20Ball (Utilities|Casting|CastToWizardmanMagicBall _array_element))))) 2.0)
          (CallFunction|DoAbsorbOneMagicBall (.AsWizardman%20Magic%20Ball (Utilities|Casting|CastToWizardmanMagicBall _array_element)))
          (Default|CallMagicBallAbsorbed (.AsWizardman%20Magic%20Ball (Utilities|Casting|CastToWizardmanMagicBall _array_element)))
          (else
            (Transformation|SetActorLocation (.AsWizardman%20Magic%20Ball (Utilities|Casting|CastToWizardmanMagicBall _array_element)) (+ (Transformation|GetActorLocation (.AsWizardman%20Magic%20Ball (Utilities|Casting|CastToWizardmanMagicBall _array_element))) (* (Math|Vector|Normalize (- (Transformation|GetWorldLocation (Variables|Default|GetAbsorbSphere)) (Transformation|GetActorLocation (.AsWizardman%20Magic%20Ball (Utilities|Casting|CastToWizardmanMagicBall _array_element))))) (/ (* DeltaSeconds 1e+03) (Math|Vector|VectorLength (- (Transformation|GetWorldLocation (Variables|Default|GetAbsorbSphere)) (Transformation|GetActorLocation (.AsWizardman%20Magic%20Ball (Utilities|Casting|CastToWizardmanMagicBall _array_element)))))))) false false)))))))

(fn ConstructionScript)