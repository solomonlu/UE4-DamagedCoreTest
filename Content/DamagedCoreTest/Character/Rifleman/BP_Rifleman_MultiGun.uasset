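; Rifleman multi-gun Blueprint that holds a shotgun and a rocket launcher and controls which one is visible.
; Each weapon hangs under its own root component, and switching hides one root and shows the other, propagated to children.
; Events select either gun explicitly or toggle by inverting both hidden states.
; The construction script makes the shotgun the default visible weapon.
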(event Custom|SwitchToRocketLauncher
  (Development|SetHiddeninGame (Variables|Default|GetRocketLauncherRoot) false true)
  (Development|SetHiddeninGame (Variables|Default|GetShotgunRoot) true true))

(event Custom|SwitchToShotGun
  (Development|SetHiddeninGame (Variables|Default|GetRocketLauncherRoot) true true)
  (Development|SetHiddeninGame (Variables|Default|GetShotgunRoot) false true))

(event Custom|ToggleGun
  (Development|SetHiddeninGame (Variables|Default|GetRocketLauncherRoot) (not (Variables|/Script/Engine.SceneComponent|GetbHiddenInGame (Variables|Default|GetRocketLauncherRoot))) true)
  (Development|SetHiddeninGame (Variables|Default|GetShotgunRoot) (not (Variables|/Script/Engine.SceneComponent|GetbHiddenInGame (Variables|Default|GetShotgunRoot))) true))

(fn ConstructionScript
  ;[1 1 1] default is shotgun
  (Development|SetHiddeninGame (Variables|Default|GetRocketLauncherRoot) true true)
  (Development|SetHiddeninGame (Variables|Default|GetShotgunRoot) false true))