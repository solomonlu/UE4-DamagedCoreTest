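; Global skill actor that makes every facility of the local player's camp invincible for a short, fixed time.
; On BeginPlay it takes the player's observe-sphere pawn out of skill spell mode, turns invincibility on, then reverts it after a delay and destroys itself.
; A helper scans all BP_FacilitiesBase actors on each toggle and sets the flag on those whose Camp matches player controller 0's.
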(event EventBeginPlay
  (|CallParentFunction)
  (bind _asbp_observe_sphere (Utilities|Casting|CastToBP_ObserveSphere (Game|Player|GetPlayerPawn 0)))
  (Default|SetinGlobalSkillSpellMode _asbp_observe_sphere false)
  (CallFunction|SetAllMyCampFacilityisInvincible true)
  (Utilities|FlowControl|Delay 8.0)
  (CallFunction|SetAllMyCampFacilityisInvincible false)
  (Actor|DestroyActor))

(fn ConstructionScript)

(fn SetAllMyCampFacilityisInvincible
  (params (IsInvincible :type Boolean))
  (bind _outactors (Actor|GetAllActorsOfClass "/Game/DamagedCoreTest/Facilities/BP_FacilitiesBase.BP_FacilitiesBase_C"))
  (for _array_element _outactors
    (if (Utilities|Enum|Equal(Enum) (Variables|/Game/DamagedCoreTest/Facilities/BP_FacilitiesBase.BP_FacilitiesBase_C|GetCamp _array_element) (Variables|/Game/DamagedCoreTest/GameMode/BP_CampPlayerController.BP_CampPlayerController_C|GetCamp (.AsBP%20Camp%20Player%20Controller (Utilities|Casting|CastToBP_CampPlayerController (Game|GetPlayerController 0)))))
      (Default|SetInvincible _array_element IsInvincible))))