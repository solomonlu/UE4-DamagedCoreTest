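; Global skill actor for a thrown ball that splits into smaller SplitBall actors, named as a soldier-spawning skill.
; On BeginPlay it sits in front of the observe sphere's camera; Throw detaches it and applies a physics impulse.
; Construction precomputes evenly spaced horizontal directions, despite the "Random" variable name.
; Once it drops below a fixed height, it spawns scaled-down balls inheriting its velocity plus those outward offsets, then destroys itself.
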(event EventBeginPlay
  (|CallParentFunction)
  (bind _asbp_observe_sphere (Utilities|Casting|CastToBP_ObserveSphere (Game|Player|GetPlayerPawn 0)))
  (Transformation|SetActorLocation (Math|Transform|TransformLocation (Transformation|GetWorldTransform (Variables|/Game/DamagedCoreTest/ObserveSphere/BP_ObserveSphere.BP_ObserveSphere_C|GetCamera _asbp_observe_sphere)) "50.000000,0.000000,20.000000") false false))

(event EventTick
  (params (DeltaSeconds :type Float%20%28single-precision%29))
  (bind _returnvalue (Transformation|GetActorTransform))
  (if (< (.z (Transformation|GetActorLocation)) 4e+02)
    (Utilities|FlowControl|DoOnce false
      (:Completed
        (bind _returnvalue_2 (Physics|GetPhysicsLinearVelocity (Variables|Default|GetSphere) "None"))
        (while (> (Variables|Default|GetCurSplitBallCount) 0)
          (Math|Integer|DecrementInt (Variables|Default|GetCurSplitBallCount)
            (:%20%20
              (Game|SpawnActorfromClass "/Game/DamagedCoreTest/GlobalSkill/BP_GlobalSkill_SpawnSoldiers_SplitBall.BP_GlobalSkill_SpawnSoldiers_SplitBall_C" (Math|Transform|MakeTransform (.location _returnvalue) (.rotation _returnvalue) (/ (.scale _returnvalue) (Math|Conversions|ToFloat(Integer) (Variables|Default|GetSplitBallCount)))) "AlwaysSpawn" 0 (+ _returnvalue_2 (* (Utilities|Array|Get(acopy) (Variables|Default|GetRandomSplitBallVector) (Variables|Default|GetCurSplitBallCount)) 400)) 0))))
        (Actor|DestroyActor)))))

(event EventThrow
  (params (ThrowVelocity :type Vector))
  (bind _sphere (Variables|Default|GetSphere))
  (Transformation|DetachFromActor self "KeepWorld" "KeepWorld" "KeepWorld")
  (Physics|SetSimulatePhysics _sphere true)
  (Physics|AddImpulseatLocation _sphere ThrowVelocity (Transformation|GetWorldLocation _sphere) "None"))

(fn ConstructionScript
  (bind _output_get (Variables|Default|SetCurSplitBallCount (Variables|Default|GetSplitBallCount)))
  (Variables|Default|SetSplitAngular (Math|Conversions|ToFloat(Integer) (/ 360 (Variables|Default|GetSplitBallCount))))
  (while (> _output_get 0)
    (bind _result (Math|Integer|DecrementInt (Variables|Default|GetCurSplitBallCount))
      (:%20%20
        (Utilities|Array|Add (Variables|Default|GetRandomSplitBallVector) (Math|Vector|MakeVector (Math|Trig|Cos(Degrees) (* _result (Variables|Default|GetSplitAngular))) (Math|Trig|Sin(Degrees) (* _result (Variables|Default|GetSplitAngular))) 0.0)))))
  (Variables|Default|SetCurSplitBallCount (Variables|Default|GetSplitBallCount)))