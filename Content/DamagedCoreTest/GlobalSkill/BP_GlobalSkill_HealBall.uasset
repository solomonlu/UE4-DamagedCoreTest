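; BP_GlobalSkill_HealBall is a throwable skill ball that becomes a temporary healing zone for controllable characters.
; On BeginPlay it moves just in front of the observe-sphere pawn's camera; Throw detaches it and launches it with a physics impulse.
; Hitting a Floor-tagged actor stops physics, swaps the ball for a range mesh and starts a short lifespan.
; Tick accumulates time to periodically heal characters found by a sphere overlap.
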(event OnComponentHit(Sphere)
  (params (HitComponent :type Primitive%20Component%20Object%20Reference) (OtherActor :type Actor%20Object%20Reference) (OtherComp :type Primitive%20Component%20Object%20Reference) (NormalImpulse :type Vector :default "0, 0, 0") (Hit :type Hit%20Result%20Structure%20%28by%20ref%29))
  (if (Utilities|Enum|Equal(Enum) (Utilities|String|ToString(Name) (Utilities|Array|Get(acopy) (Variables|/Script/Engine.Actor|GetTags OtherActor))) "Floor")
    (Physics|SetSimulatePhysics (Variables|Default|GetSphere) false)
    (Variables|Default|SetIsHealing true)
    (Actor|SetLifeSpan 5.0)
    (Development|SetHiddeninGame (Variables|Default|GetHealRangeMesh) false false)
    (Development|SetHiddeninGame (Variables|Default|GetStaticMesh) true false)
    (Transformation|SetActorRotation "0, 0, 0")))

(event EventBeginPlay
  (|CallParentFunction)
  (bind _asbp_observe_sphere (Utilities|Casting|CastToBP_ObserveSphere (Game|Player|GetPlayerPawn 0)))
  (Transformation|SetActorLocation (Math|Transform|TransformLocation (Transformation|GetWorldTransform (Variables|/Game/DamagedCoreTest/ObserveSphere/BP_ObserveSphere.BP_ObserveSphere_C|GetCamera _asbp_observe_sphere)) "100.000000,0.000000,20.000000") false false))

(event EventTick
  (params (DeltaSeconds :type Float%20%28single-precision%29))
  (if (Variables|Default|GetIsHealing)
    (Variables|Default|SetCurHealingTick (+ DeltaSeconds (Variables|Default|GetCurHealingTick)))
    (if (> (Variables|Default|GetCurHealingTick) (Variables|Default|GetHealingTick))
      (Variables|Default|SetCurHealingTick (- (Variables|Default|GetCurHealingTick) (Variables|Default|GetHealingTick)))
      (bind _outactors (Class|KismetSystemLibrary|SphereOverlapActorsNEW (Transformation|GetActorLocation) (Variables|Default|GetHealRange) (Utilities|Array|MakeArray "ObjectTypeQuery2") "/Game/DamagedCoreTest/Character/BP_ControllableCharacter_Base.BP_ControllableCharacter_Base_C"))
      (for _array_element _outactors
        (Default|Heal (.AsBP%20Controllable%20Character%20Base (Utilities|Casting|CastToBP_ControllableCharacter_Base _array_element)) (Variables|Default|GetHealingHealth))))))

(event EventThrow
  (params (ThrowVelocity :type Vector))
  (bind _sphere (Variables|Default|GetSphere))
  (Transformation|DetachFromActor self "KeepWorld" "KeepWorld" "KeepWorld")
  (Physics|SetSimulatePhysics _sphere true)
  (Physics|AddImpulseatLocation _sphere ThrowVelocity (Transformation|GetWorldLocation _sphere) "None"))

(fn ConstructionScript)