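; Global Focus Fire skill actor that lets the player mark an enemy character by aiming the right motion controller of BP_ObserveSphere.
; On BeginPlay it attaches to that controller, then each tick sphere-traces forward for a controllable character outside the player's camp.
; While a target is held, TracingBall advances along local X toward it, and retracts when the target is lost.
; Once the ball covers the distance, it calls SetBeFocusFire on the target and destroys itself.
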(event EventBeginPlay
  (|CallParentFunction)
  (bind _asbp_observe_sphere (Utilities|Casting|CastToBP_ObserveSphere (Game|Player|GetPlayerPawn 0)))
  (Transformation|AttachComponentToComponent (Variables|/Game/DamagedCoreTest/ObserveSphere/BP_ObserveSphere.BP_ObserveSphere_C|GetRightMotionController _asbp_observe_sphere) "None" "KeepRelative" "KeepRelative" "KeepWorld" true)
  (Transformation|SetActorRelativeLocation "0, 0, 0")
  (Transformation|SetActorRelativeRotation "0, 0, 0"))

(event EventTick
  (params (DeltaSeconds :type Float%20%28single-precision%29))
  (bind _returnvalue (Transformation|GetActorLocation))
  (Utilities|FlowControl|Sequence
    (:then_0
      ;[1 1 1] get tracing actor
      (bind _outactors (Actor|GetAllActorsOfClass "/Game/DamagedCoreTest/ObserveSphere/BP_ObserveSphere.BP_ObserveSphere_C"))
      (bind _outhit (Collision|SphereTraceForObjects _returnvalue (+ _returnvalue (* (Transformation|GetActorForwardVector) 5e+03)) 15.0 (Utilities|Array|MakeArray "ObjectTypeQuery2") false _outactors "None"))
      (if (Utilities|IsValid (.HitActor (Collision|BreakHitResult _outhit)))
        (bind _asbp_controllable_character_base (Utilities|Casting|CastToBP_ControllableCharacter_Base (.HitActor (Collision|BreakHitResult _outhit)))
          (:then
            (bind _asbp_camp_player_controller (Utilities|Casting|CastToBP_CampPlayerController (Game|GetPlayerController 0))
              (:then
                (if (Utilities|Enum|NotEqual(Enum) (Variables|/Game/DamagedCoreTest/Character/BP_ControllableCharacter_Base.BP_ControllableCharacter_Base_C|GetCamp _asbp_controllable_character_base) (Variables|/Game/DamagedCoreTest/GameMode/BP_CampPlayerController.BP_CampPlayerController_C|GetCamp _asbp_camp_player_controller))
                  (Variables|Default|SetIsTracing true)
                  (Variables|Default|SetTracingActor _asbp_controllable_character_base)
                  (else
                    (Variables|Default|SetIsTracing false :!label _label)
                    (Variables|Default|SetTracingActor 0))))
              (:CastFailed
                (goto _label))))
          (:CastFailed
            (goto _label)))
        (else
          (goto _label))))
    (:then_1
      ;[1 1 1] move trace ball
      (if (and (Variables|Default|GetIsTracing) (Utilities|IsValid (Variables|Default|GetTracingActor)))
        (if (< (.x (Variables|/Script/Engine.SceneComponent|GetRelativeLocation (Variables|Default|GetTracingBall))) (Transformation|GetDistanceTo (Variables|Default|GetTracingActor) self))
          (Transformation|AddRelativeLocation (Variables|Default|GetTracingBall) (Math|Vector|MakeVector (* DeltaSeconds (Variables|Default|GetTraceToSpeed)) 0.0 0.0) false false)
          (else
            (Utilities|FlowControl|DoOnce false
              (:Completed
                ;;[1 1 1] trace complete
                (Default|SetbeFocusFire (Variables|Default|GetTracingActor))
                (Actor|DestroyActor)))))
        (elif (> (.x (Variables|/Script/Engine.SceneComponent|GetRelativeLocation (Variables|Default|GetTracingBall))) 0.0)
          (Transformation|AddRelativeLocation (Variables|Default|GetTracingBall) (Math|Vector|MakeVector (* DeltaSeconds (Variables|Default|GetTraceBackSpeed) -1.0) 0.0 0.0) false false))))))

(fn ConstructionScript)