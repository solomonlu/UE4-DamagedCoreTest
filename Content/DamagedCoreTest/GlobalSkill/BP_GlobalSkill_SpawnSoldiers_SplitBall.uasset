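; Projectile for a spawn-soldiers global skill that turns into an AI bowman where it lands.
; The construction script feeds InitVelocity into the projectile movement component.
; When the mesh hits an actor whose first tag is Floor, it spawns a Bowman_Character at the impact with the first player controller's Camp.
; The bowman gets a default AI controller, then the ball destroys itself.
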(event OnComponentHit(StaticMesh)
  (params (HitComponent :type Primitive%20Component%20Object%20Reference) (OtherActor :type Actor%20Object%20Reference) (OtherComp :type Primitive%20Component%20Object%20Reference) (NormalImpulse :type Vector :default "0, 0, 0") (Hit :type Hit%20Result%20Structure%20%28by%20ref%29))
  (if (Utilities|Enum|Equal(Enum) (Utilities|String|ToString(Name) (Utilities|Array|Get(acopy) (Variables|/Script/Engine.Actor|GetTags OtherActor))) "Floor")
    (bind _asbp_camp_player_controller (Utilities|Casting|CastToBP_CampPlayerController (Game|GetPlayerController 0)))
    (bind _returnvalue (Game|SpawnActorfromClass "/Game/DamagedCoreTest/Character/Bowman/Bowman_Character.Bowman_Character_C" (Math|Transform|MakeTransform (.Location (Collision|BreakHitResult Hit)) "0, 0, 0" "1,1,1") "Undefined" 0 (Variables|/Game/DamagedCoreTest/GameMode/BP_CampPlayerController.BP_CampPlayerController_C|GetCamp _asbp_camp_player_controller) 0))
    (bind _defaultaicontroller (Default|SpawnDefaultAIController _returnvalue))
    (Pawn|Possess _defaultaicontroller _returnvalue)
    (Actor|DestroyActor)))

(event EventBeginPlay)

(fn ConstructionScript
  (Variables|/Script/Engine.MovementComponent|SetVelocity (Variables|Default|GetProjectileMovement) (Variables|Default|GetInitVelocity)))