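; Boomerang component that flies its owning actor out along a curved path and back to a returning scene component.
; ThrowOut seeds decaying throw and fly vectors, which Tick sums into swept movement with velocity-based spin.
; Aligning with the target direction flips the throw arc and aims back, or starts straight homing if already flagged.
; WorldStatic hits also trigger straight homing; arrival near the return point destroys the owner after a delay.
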(event Custom|ThrowOut
  (params (ProjectedVector%28Throw%29 :type Vector) (TargetPos%28Fly%29 :type Vector) (ReturningSceneComp :type Scene%20Component%20Object%20Reference) (ControlerVector :type Vector) (ThrowScale :type Float%20%28single-precision%29) (FlyScale :type Float%20%28single-precision%29) (FlyLimit :type Vector%202D%20Structure))
  (bind _returnvalue (Math|Vector|VectorLength ProjectedVector%28Throw%29))
  (bind _returnvalue_2 (Components|GetOwner))
  (bind _returnvalue_3 (Math|Vector|VectorLength TargetPos%28Fly%29))
  (bind _returnvalue_4 (Transformation|GetActorLocation _returnvalue_2))
  (bind _returnvalue_5 (* _returnvalue (Variables|Default|GetThrowScale)))
  (bind _returnvalue_6 (* _returnvalue_3 (Variables|Default|GetFlyScale)))
  ;[1 0.3229 0.739] StartFromHere
  (Utilities|FlowControl|Sequence
    (:then_0
      (CallFunction|UpdateScales ThrowScale FlyScale)
      (Variables|Default|SetFlyLimit FlyLimit))
    (:then_1
      (Variables|Private|SetVelocityThrow _returnvalue_5)
      (Variables|Private|SetThrowDir (+ (Math|Vector|Normalize TargetPos%28Fly%29) (* ControlerVector 5.0)))
      (Variables|Private|SetVelocityThrow_0 _returnvalue_5))
    (:then_2
      (Variables|Private|SetFlyDir (Math|Vector|Normalize (+ (* (Math|Vector|Normalize TargetPos%28Fly%29) 5.0) ControlerVector)))
      (Variables|Private|SetVelocityFly _returnvalue_6)
      (Variables|Private|SetVelocityFly_0 _returnvalue_6))
    (:then_3
      (Variables|Private|SetStartingPos (Transformation|GetActorLocation (Components|GetOwner))))
    (:then_4
      (Variables|Private|SetStatusByte 1)
      (CallFunction|ResetReturningPoint)
      (CallFunction|ResetDIstanceCheck)
      (CallFunction|ResetBumpandBack))
    (:then_5
      ;[1 1 1] Debug
      (if (Variables|Default|GetIsDebug)
        (Utilities|FlowControl|Sequence
          (:then_0
            ;;[1 0.2831 0.9387] Draw Throw
            (Rendering|Debug|DrawDebugLine _returnvalue_4 (+ (* (Variables|Private|GetThrowDir) (Variables|Private|GetVelocityThrow)) _returnvalue_4) "(R=1.000000,G=0.283140,B=0.933837,A=1.000000)" 1e+02 3.0))
          (:then_1
            ;;[0.2195 0.3864 1] Draw Fly
            (Rendering|Debug|DrawDebugLine _returnvalue_4 (+ _returnvalue_4 TargetPos%28Fly%29) "(R=0.218681,G=0.385869,B=1.000000,A=1.000000)" 1e+02 3.0)))))))

(event Custom|ResetBumpAndBack
  (Utilities|FlowControl|DoOnce false) ; enters at Reset
)

(event Custom|ResetReturningPoint
  ;[0.1144 1 0.9911] If Homing
  (Utilities|FlowControl|DoOnce false) ; enters at Reset
)

(event Custom|StraitToHand
  ;[0.1144 1 0.9911] Homing
  ;;[0.9522 1 0] Line Homing Trigger
  (Variables|Private|SetFlyDir (Class|KismetMathLibrary|GetDirectionVector (Transformation|GetActorLocation (Components|GetOwner)) (Transformation|GetWorldLocation (stale Custom|ThrowOut ReturningSceneComp))))
  (Variables|Private|SetThrowFactor 0.0)
  (Variables|Default|SetIsLineHoming true)
  (Variables|Private|SetStatusByte 2))

(event Custom|ResetDIstanceCheck
  (Utilities|FlowControl|DoOnce false) ; enters at Reset
)

(event EventTick
  (params (DeltaSeconds :type Float%20%28single-precision%29))
  (bind _returnvalue (Components|GetOwner))
  (bind _flylimit (Variables|Default|GetFlyLimit))
  (bind _flylimit_2 (Variables|Default|GetFlyLimit))
  (bind _returnvalue_2 (Transformation|GetActorLocation _returnvalue))
  (bind (_x _y) (Math|Vector2D|BreakVector2D _flylimit_2))
  (bind (_x_2 _y_2) (Math|Vector2D|BreakVector2D _flylimit))
  ;[1 1 1] =0 None; =1 Thrown; =2 Returning
  (switch int (Variables|Private|GetStatusByte)
    (:1
      (Utilities|FlowControl|Sequence :!label _label
        (:then_0
          ;[0.1144 1 0.9911] Movement
          (bind _sweephitresult (Transformation|AddActorWorldOffset (Components|GetOwner) (+ (* (Variables|Private|GetFlyDir) (* DeltaSeconds (Math|Float|Clamp(Float) (Math|Float|Absolute(Float) (Variables|Private|GetVelocityFly)) _x _y) 5.0)) (* (Variables|Private|GetThrowDir) (* DeltaSeconds (Variables|Private|GetVelocityThrow) 1e+01 (Variables|Private|GetThrowFactor)))) true))
          (if (.bBlockingHit (Collision|BreakHitResult _sweephitresult))
            (if (Utilities|Enum|Equal(Enum) (Collision|GetCollisionObjectType (.HitComponent (Collision|BreakHitResult _sweephitresult))) "ECC_WorldStatic")
              (Utilities|FlowControl|DoOnce false
                (:Completed
                  (CallFunction|StraittoHand))))))
        (:then_1
          ;[0.1144 1 0.9911] Reduce speed with frame rate
          (Variables|Private|SetVelocityThrow (- (Variables|Private|GetVelocityThrow) (* DeltaSeconds 6e+01))))
        (:then_2
          (Variables|Private|SetVelocityFly (- (Variables|Private|GetVelocityFly) (* DeltaSeconds 1e+02))))
        (:then_3
          ;[0.1144 1 0.9911] Spin as per Velocity
          (Transformation|AddActorLocalRotation (Components|GetOwner) (Math|Rotator|MakeRotator 0.0 0.0 (Math|Float|Clamp(Float) (Math|Float|Absolute(Float) (/ (Variables|Private|GetVelocityThrow) 1e+01)) _x_2 _y_2)) false false))
        (:then_4
          ;[0.1144 1 0.9911] If Homing
          (if (Math|Vector|Equal(Vector) (Math|Vector|Normalize (- (Transformation|GetActorLocation (Components|GetOwner)) (Variables|Private|GetStartingPos))) (Math|Vector|Normalize (stale Custom|ThrowOut TargetPos%28Fly%29)) 0.1)
            (Utilities|FlowControl|DoOnce false
              (:Completed
                (if (Variables|Default|GetIsLineHoming)
                  (Utilities|FlowControl|Delay (Math|Random|RandomFloatinRange 0.05 0.3))
                  (CallFunction|StraittoHand)
                  (else
                    (Variables|Private|SetThrowFactor (* (Variables|Private|GetThrowFactor) -1.0))
                    (Variables|Private|SetFlyDir (Class|KismetMathLibrary|GetDirectionVector (Transformation|GetActorLocation (Components|GetOwner)) (Transformation|GetWorldLocation (stale Custom|ThrowOut ReturningSceneComp))))
                    (Variables|Private|SetStatusByte 2)
                    (Variables|Private|SetVelocityFly (Variables|Private|GetVelocityFly_0))
                    (Variables|Private|SetVelocityThrow (Variables|Private|GetVelocityThrow_0))))))))
        (:then_5
          ;[0.1144 1 0.9911] Homing
          (if (Variables|Default|GetIsLineHoming)
            (if (== (Variables|Private|GetStatusByte) 2)
              (Variables|Private|SetFlyDir (Class|KismetMathLibrary|GetDirectionVector (Transformation|GetActorLocation (Components|GetOwner)) (Transformation|GetWorldLocation (stale Custom|ThrowOut ReturningSceneComp)))))))
        (:then_6
          ;[1 1 1] Debug
          (if (Variables|Default|GetIsDebug)
            ;;[0.9823 1 0] Debug Trace
            (Utilities|FlowControl|Sequence
              (:then_0
                (Rendering|Debug|DrawDebugPoint (Transformation|GetActorLocation (Components|GetOwner)) 2.0 "(R=0.981443,G=1.000000,B=0.000000,A=1.000000)" 1e+02))
              (:then_1
                ;;[0 0.003035 1] Debug Fly Dir
                (Rendering|Debug|DrawDebugLine _returnvalue_2 (+ _returnvalue_2 (* (Variables|Private|GetFlyDir) 3e+01)) "(R=0.000000,G=0.003194,B=1.000000,A=1.000000)" 1e+02 1.0)))))))
    (:2
      (Utilities|FlowControl|Sequence
        (:then_0
          (goto _label))
        (:then_1
          (if (<= (Math|Vector|VectorLength (- (Transformation|GetActorLocation (Components|GetOwner)) (Transformation|GetWorldLocation (stale Custom|ThrowOut ReturningSceneComp)))) 1.2e+02)
            (Utilities|FlowControl|DoOnce false
              (:Completed
                (CallFunction|StraittoHand)
                (Utilities|FlowControl|Delay 1.0)
                (Actor|DestroyActor (Components|GetOwner))))))))))

(fn UpdateScales
  (params (ThrowScale :type Float%20%28single-precision%29) (FlyScale :type Float%20%28single-precision%29))
  (Utilities|FlowControl|Sequence
    (:then_0
      (if (and (> ThrowScale 0.0) (!= ThrowScale (Variables|Default|GetThrowScale)))
        (Variables|Default|SetThrowScale ThrowScale)))
    (:then_1
      (if (and (> FlyScale 0.0) (!= FlyScale (Variables|Default|GetFlyScale)))
        (Variables|Default|SetFlyScale FlyScale)))))