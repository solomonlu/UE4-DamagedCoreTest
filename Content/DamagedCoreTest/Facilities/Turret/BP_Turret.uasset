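; BP_Turret is a turret facility that fires TurretProjectile actors on a cooldown.
; Tick counts the cooldown down, and CanFire allows a shot only when the turret is alive and the cooldown has elapsed.
; Fire resets the cooldown and spawns an enlarged projectile at the tip of the Arrow component, matching its rotation, with the turret as owner and instigator.
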(event Custom|Fire!
  (bind _self self)
  (bind _arrow (Variables|Default|GetArrow))
  (bind _returnvalue (Transformation|GetWorldRotation _arrow))
  (Variables|Default|SetCurFireCoolDown (Variables|Default|GetFireCoolDown))
  (Game|SpawnActorfromClass "/Game/DamagedCoreTest/Weapon/Bullet/TurretProjectile.TurretProjectile_C" (Math|Transform|MakeTransform (+ (Transformation|GetWorldLocation _arrow) (* (Math|Vector|GetForwardVector _returnvalue) (* (Variables|/Script/Engine.ArrowComponent|GetArrowSize _arrow) 8e+01))) _returnvalue "2.000000,2.000000,2.000000") "Undefined" _self _self))

(event EventTick
  (params (DeltaSeconds :type Float%20%28single-precision%29))
  (if (> (Variables|Default|GetCurFireCoolDown) 0.0)
    (Variables|Default|SetCurFireCoolDown (- (Variables|Default|GetCurFireCoolDown) DeltaSeconds))))

(fn ConstructionScript
  (|CallParentFunction))

(fn CanFire
  (return (and (not (Variables|Default|GetIsDead)) (<= (Variables|Default|GetCurFireCoolDown) 0.0))))