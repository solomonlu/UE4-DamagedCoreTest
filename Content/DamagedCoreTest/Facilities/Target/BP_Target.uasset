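; BP_Target is a target facility that takes damage through its parent class and regenerates health after a delay without hits.
; Tick counts time since the last damage and, past the recovery limit, opens a Gate that adds HPRecoverSpeed every frame, unscaled by delta time, clamped to MaxHealth.
; Taking damage resets the timer and closes the Gate, as does reaching full health.
; OnDeath is deliberately left empty.
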(event EventOnDeath
  ;[1 1 1] do nothing is good
)

(event EventTick
  (params (DeltaSeconds :type Float%20%28single-precision%29))
  (Utilities|FlowControl|Sequence
    (:then_0
      (if (< (Variables|Default|GetCurHealth) (Math|Conversions|ToFloat(Integer) (Variables|Default|GetMaxHealth)))
        (bind _output_get (Variables|Default|SetCurRecoverTime (+ (Variables|Default|GetCurRecoverTime) DeltaSeconds)))
        (if (>= _output_get (Variables|Default|GetRecoverLimitTime))
          (goto _label Open))
        (else
          (goto _label Close))))
    (:then_1
      (Utilities|FlowControl|Gate true :!label _label
        (:Exit
          (Variables|Default|SetCurHealth (Math|Float|Clamp(Float) (+ (Variables|Default|GetCurHealth) (Variables|Default|GetHPRecoverSpeed)) 0.0 (Math|Conversions|ToFloat(Integer) (Variables|Default|GetMaxHealth)))))))))

(event Game|Damage|EventAnyDamage
  (params (Damage :type Float%20%28single-precision%29) (DamageType :type Damage%20Type%20Object%20Reference) (InstigatedBy :type Controller%20Object%20Reference) (DamageCauser :type Actor%20Object%20Reference))
  (|CallParentFunction Damage DamageType InstigatedBy DamageCauser)
  (Variables|Default|SetCurRecoverTime 0.0)
  (Utilities|FlowControl|Gate true) ; enters at Close
)

(fn ConstructionScript
  (|CallParentFunction))