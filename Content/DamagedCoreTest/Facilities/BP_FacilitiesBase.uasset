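; Base Blueprint for a damageable facility with health, an invincibility state shown by an effect, and a health text indicator.
; AnyDamage lowers clamped health unless dead or invincible, spawning a floating damage tip when a locally controlled pawn caused the hit.
; At zero health it expires after a short lifespan and switches its connected observer sphere's camp.
; A CurHealth RepNotify and the construction script refresh the indicator text.
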(event Custom|OnDeath
  (bind _connectedobserversphere (Variables|Default|GetConnectedObserverSphere))
  (Actor|SetLifeSpan 0.5)
  (Utilities|IsValid _connectedobserversphere
    (:Is%20Valid
      (Variables|/Game/DamagedCoreTest/ObserveSphere/BP_ObserveSphere.BP_ObserveSphere_C|SetCamp _connectedobserversphere "NewEnumerator2"))))

(event Custom|SetInvincible
  (params (IsInvincible :type Boolean))
  (bind _output_get (Variables|Default|SetIsInvincible IsInvincible))
  (Development|SetHiddeninGame (Variables|Default|GetInvincibleEffect) (not _output_get) false))

(event Game|Damage|EventAnyDamage
  (params (Damage :type Float%20%28single-precision%29) (DamageType :type Damage%20Type%20Object%20Reference) (InstigatedBy :type Controller%20Object%20Reference) (DamageCauser :type Actor%20Object%20Reference))
  (bind (_aspawn _bsuccess) (Utilities|Casting|CastToPawn DamageCauser))
  (if (not (or (Variables|Default|GetIsDead) (Variables|Default|GetIsInvincible)))
    (bind _output_get (Variables|Default|SetCurHealth (Math|Float|Clamp(Float) (- (Variables|Default|GetCurHealth) Damage) 0.0 (Math|Conversions|ToFloat(Integer) (Variables|Default|GetMaxHealth)))))
    (if (Math|Boolean|ANDBoolean (Utilities|IsValid DamageCauser) _bsuccess (Pawn|IsLocalPlayerController (Pawn|GetController _aspawn)))
      (Game|SpawnActorfromClass "/Game/DamagedCoreTest/Gizmos/BP_HealthChangeTips.BP_HealthChangeTips_C" (Math|Transform|MakeTransform (+ (Transformation|GetWorldLocation (Variables|Default|GetHealthIndicator)) "0, 0,20.000000") "0, 0, 0" "1,1,1") "Undefined" 0 (* -1 Damage) _aspawn))
    (if (<= _output_get 0.0)
      (CallFunction|OnDeath))))

(fn ConstructionScript
  (Rendering|Components|TextRender|SetText (Variables|Default|GetHealthIndicator) (Utilities|Text|ToText(String) (Utilities|String|Append (Utilities|String|ToString(Integer) (Math|Float|Truncate (Variables|Default|GetCurHealth))) "/" (Utilities|String|ToString(Integer) (Variables|Default|GetMaxHealth))))))

(fn OnRepCurHealth
  (Rendering|Components|TextRender|SetText (Variables|Default|GetHealthIndicator) (Utilities|Text|ToText(String) (Utilities|String|Append (Utilities|String|ToString(Integer) (Math|Float|Truncate (Variables|Default|GetCurHealth))) "/" (Utilities|String|ToString(Integer) (Variables|Default|GetMaxHealth))))))