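; BP_Barracks is a facility that periodically spawns AI soldiers for its Camp.
; BeginSpawnSoldies spawns a wave immediately and starts a looping timer, which StopSpawnSoldies clears.
; Each wave places one random soldier class at every actor-relative SpawnLocation, with a look-at rotation, then spawns a controller to possess it.
; The controller uses the stored LastSoldierClassIndex, while the soldier class rolls its own random index, so the pair can mismatch.
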(event Custom|SpawnSoldies
  (if (Variables|Default|GetCanSpawnSoldiers)
    (for _array_element (Variables|Default|GetSpawnLocations)
      (|SpawnSingleSoldier _array_element))))

(event Custom|StopSpawnSoldies
  (Variables|Default|SetCanSpawnSoldiers false)
  (Utilities|Time|ClearandInvalidateTimerbyHandle (Variables|Default|GetSpawnHandle)))

(event Custom|BeginSpawnSoldies
  (Variables|Default|SetCanSpawnSoldiers true)
  (CallFunction|SpawnSoldies)
  (bind _returnvalue (Utilities|Time|SetTimerbyEvent (delegate Custom|SpawnSoldies) (Variables|Default|GetSpawnSoldiersInterval) true))
  (Variables|Default|SetSpawnHandle _returnvalue))

(fn ConstructionScript
  (|CallParentFunction))