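; BP_HealthChangeTips is a world-space text actor that displays a health change amount.
; The construction script writes HealthChangeValue into the TipsRender text component, colored green for positive values and red otherwise.
; Each tick the whole actor rotates toward the FaceToPawn actor's location, acting as a billboard for that pawn.
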(event EventBeginPlay)

(event Collision|EventActorBeginOverlap
  (params (OtherActor :type Actor%20Object%20Reference)))

(event EventTick
  (params (DeltaSeconds :type Float%20%28single-precision%29))
  (Transformation|SetActorRotation (Math|Rotator|FindLookatRotation (Transformation|GetActorLocation) (Transformation|GetActorLocation (Variables|Default|GetFaceToPawn)))))

(fn ConstructionScript
  (Utilities|FlowControl|Sequence
    (:then_0
      (Rendering|Components|TextRender|SetText (Variables|Default|GetTipsRender) (Utilities|Text|ToText(Float) (Variables|Default|GetHealthChangeValue) "HalfToEven"))
      (if (> (Variables|Default|GetHealthChangeValue) 0.0)
        (bind _output_get (Variables|Default|SetColor "(R=0.000000,G=1.000000,B=0.000000,A=1.000000)"))
        (Rendering|Components|TextRender|SetTextRenderColor (Variables|Default|GetTipsRender) (Math|Conversions|ToColor(LinearColor) _output_get))
        (else
          (bind _output_get_2 (Variables|Default|SetColor "(R=1.000000,G=0.000000,B=0.000000,A=1.000000)"))
          (Rendering|Components|TextRender|SetTextRenderColor (Variables|Default|GetTipsRender) (Math|Conversions|ToColor(LinearColor) _output_get_2)))))))