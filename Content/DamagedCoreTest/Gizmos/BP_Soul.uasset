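; BP_Soul is a soul gizmo actor that drifts skyward after spawning, then flies to the player and destroys itself on arrival.
; For five seconds, Tick applies a mostly upward random offset, re-rolled after a random number of ticks, so the drift is frame-rate dependent.
; A delayed flag from BeginPlay then switches Tick to delta-time-scaled homing on player pawn 0, without sweeping, until it comes within a small radius.
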(event EventBeginPlay
  (Utilities|FlowControl|Delay 5.0)
  (Variables|Default|SetIsFlyToPlayer true))

(event EventTick
  (params (DeltaSeconds :type Float%20%28single-precision%29))
  (bind _returnvalue (Transformation|GetActorLocation))
  (bind _returnvalue_2 (Game|Player|GetPlayerPawn 0))
  (bind _returnvalue_3 (Transformation|GetActorLocation _returnvalue_2))
  (bind _returnvalue_4 (- _returnvalue_3 _returnvalue))
  (if (Variables|Default|GetIsFlyToPlayer)
    ;[1 1 1] second fly to player
    (Transformation|AddActorWorldOffset (* (Math|Vector|Normalize _returnvalue_4) (* DeltaSeconds (Variables|Default|GetFlyToPlayerSpeed))))
    (if (< (Math|Vector|VectorLength _returnvalue_4) 5.0)
      (Actor|DestroyActor))
    (else
      ;[1 1 1] first float to sky
      (if (> (Variables|Default|GetUnChangeDirectionTickCount) 0)
        _
        (else
          (Variables|Default|SetUnChangeDirectionTickCount (Math|Random|RandomIntegerinRange 50 100))
          (Variables|Default|SetNextLocationTickOffset (Math|Vector|MakeVector (Math|Random|RandomFloatinRange -0.5 0.5) (Math|Random|RandomFloatinRange -0.5 0.5) (Math|Random|RandomFloatinRange 0.85 1.2)))))
      (Transformation|AddActorWorldOffset (Variables|Default|GetNextLocationTickOffset))
      (Math|Integer|DecrementInt (Variables|Default|GetUnChangeDirectionTickCount)))))

(fn ConstructionScript)