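; BP_LeftHandMenu is a child menu actor, apparently a left-hand test menu built on Trace widgets.
; On MenuInitialised it calls the parent, finds the TraceButton named "Button" and binds its click.
; A click spawns a tutorial particle emitter at the actor's location and destroys it after a short delay.
; A handler printing clicked TraceTable items exists, but its binding is disconnected and never runs.
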(event Custom|MenuItemClickedASD
  (params (ClickedItem :type Trace%20Table%20Item%20Object%20Reference))
  ;[1 1 1] Get the menu item that was clicked
  ;[1 1 1] If that menu item was the first one print
  (Development|PrintString (Utilities|String|Append (Utilities|String|ToString(Text) (Variables|/Game/ExampleContent/VR_Trace_Interaction/Blueprints/Widgets/BaseTraceWidgets/TraceTableItem.TraceTableItem_C|Gettext ClickedItem)) " pressed")))

(event Custom|OnClicked_Event_0
  (params (this :type Trace%20Button%20Object%20Reference))
  ;[1 1 1] Find the widget named Button in the menu and assign an event to it's onClicked method
  ;[1 1 1] Spawn emited when the button is clicked
  (bind _returnvalue (Effects|SpawnEmitteratLocation "/Engine/Tutorial/SubEditors/TutorialAssets/TutorialParticleSystem.TutorialParticleSystem" (Transformation|GetActorLocation)))
  (Utilities|FlowControl|Delay 0.5)
  (Components|DestroyComponent _returnvalue))

(event EventMenuInitialised
  (|CallParentFunction)
  ;[1 1 1] Find the widget named Button in the menu and assign an event to it's onClicked method
  (bind _widget (Class|TraceMenuInteractionInterface|GetWidgetbyName(Message) (Variables|Default|GetMenuWidget) "Button"))
  (bind _astrace_button (Utilities|Casting|CastToTraceButton _widget))
  (EventDispatchers|AssignOnClicked _astrace_button (delegate Custom|OnClicked_Event_0)))

(event EventActorBeginOverlap
  (params (OtherActor :type Actor%20Object%20Reference)))

(event EventTick
  (params (DeltaSeconds :type Float%20%28single-precision%29)))

(fn ConstructionScript
  (|CallParentFunction))