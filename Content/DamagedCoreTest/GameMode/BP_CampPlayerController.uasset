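; Player controller for camp play that manages an energy meter tied to the currently possessed pawn.
; Every tick, DealEnergy refills energy while it controls a BP_ObserveSphere and drains it while it controls a BP_ControllableCharacter_Base, clamped to the maximum.
; Once energy is empty, it calls OnEnergyExhaust on the controlled character on each tick it remains possessed.
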(event EventTick
  (params (DeltaSeconds :type Float%20%28single-precision%29))
  (Utilities|FlowControl|Sequence
    (:then_0
      (CallFunction|DealEnergy DeltaSeconds))))

(fn ConstructionScript)

(fn DealEnergy
  (params (DeltaTime :type Float%20%28single-precision%29))
  (bind _returnvalue (Pawn|GetControlledPawn))
  (Utilities|Casting|CastToBP_ObserveSphere _returnvalue
    (:then
      ;[1 1 1] on observer sphere,recover energy
      (if (< (Variables|Energy|GetCurEnergy) (Math|Conversions|ToFloat(Integer) (Variables|Energy|GetMaxEnergy)))
        (Variables|Energy|SetCurEnergy (Math|Float|Clamp(Float) (+ (Variables|Energy|GetCurEnergy) (* DeltaTime (Variables|Energy|GetEnergyRecoverSpeed))) 0.0 (Math|Conversions|ToFloat(Integer) (Variables|Energy|GetMaxEnergy)))))
      (return))
    (:CastFailed
      (bind _asbp_controllable_character_base (Utilities|Casting|CastToBP_ControllableCharacter_Base _returnvalue)
        (:then
          ;[1 1 1] on character,consume energy
          (if (> (Variables|Energy|GetCurEnergy) 0.0)
            (Variables|Energy|SetCurEnergy (Math|Float|Clamp(Float) (- (Variables|Energy|GetCurEnergy) (* DeltaTime (Variables|Energy|GetEnergyExhaustSpeed))) 0.0 (Math|Conversions|ToFloat(Integer) (Variables|Energy|GetMaxEnergy))))
            (else
              (Default|OnEnergyExhaust _asbp_controllable_character_base)))
          (return))
        (:CastFailed
          (return))))))