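; BP_BattleGameMode is a battle game mode that shuts down AI soldiers once exactly one barracks remains in the level.
; Every Tick it polls for BP_Barracks actors and, when the count is one, tells that barracks to stop spawning soldiers.
; It then destroys every Rifleman_Character not controlled by a player, repeating this each frame while the condition holds.
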(event EventBeginPlay)

(event EventTick
  (params (DeltaSeconds :type Float%20%28single-precision%29))
  (bind _outactors (Actor|GetAllActorsOfClass "/Game/DamagedCoreTest/Facilities/Barracks/BP_Barracks.BP_Barracks_C"))
  (if (== (Utilities|Array|Length _outactors) 1)
    (Default|StopSpawnSoldies (Utilities|Array|Get(acopy) _outactors))
    (bind _outactors_2 (Actor|GetAllActorsOfClass "/Game/DamagedCoreTest/Character/Rifleman/Rifleman_Character.Rifleman_Character_C"))
    (for _array_element _outactors_2
      (if (not (Pawn|IsPlayerControlled _array_element))
        (Actor|DestroyActor _array_element)))))

(fn ConstructionScript)